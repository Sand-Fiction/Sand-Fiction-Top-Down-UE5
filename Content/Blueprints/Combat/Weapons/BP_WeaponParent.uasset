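; BP_WeaponParent is a base weapon Blueprint that can dissolve and reappear visually.
; Its construction script assigns the WeaponMesh variable to the mesh component.
; On BeginPlay it creates a dynamic instance of M_WeaponDissolve and applies it to the mesh's first material slot.
; Dissolve plays a Fade timeline that drives the material's Fade parameter, and Appear plays that timeline in reverse from the end.
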(event `self.ReceiveBeginPlay`
  (bind _mesh (`self.Mesh`))
  (bind _returnvalue (`PrimitiveComponent.CreateDynamicMaterialInstance` _mesh 0 "/Game/Blueprints/Combat/Weapons/M_WeaponDissolve.M_WeaponDissolve" "None"))
  (bind _output_get (set `self.DMI` _returnvalue))
  (`PrimitiveComponent.SetMaterial` _mesh 0 _output_get))

(event `Dissolve`
  (bind (_direction _fade) (`Timeline|Fade` :!via `PlayFromStart` :!label _label)
    (:`Update`
      (`MaterialInstanceDynamic.SetScalarParameterValue` (`self.DMI`) "Fade" _fade))))

(event `Appear`
  (goto _label :!via `ReverseFromEnd`))

(fn `UserConstructionScript`
  (`StaticMeshComponent.SetStaticMesh` (`self.Mesh`) (`self.Weapon Mesh`)))