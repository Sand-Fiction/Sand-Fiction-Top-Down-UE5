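; BP_RangedProjectile is a combat projectile that damages enemy characters on impact.
; On BeginPlay, if the Shoot flag is set, it enables projectile movement simulation and starts a timed self-destruct after a fixed delay.
; When its Box component hits a Character_Enemy, it removes health through that enemy's CombatComponent and destroys itself, while hits on other actors are ignored.
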(event `self.ReceiveBeginPlay`
  (if (`self.Shoot`)
    (set `ProjectileMovementComponent.bSimulationEnabled` true (`self.ProjectileMovement`))
    (`self.DestroyAfterTime`)))

(event `DestroyAfterTime`
  (`KismetSystemLibrary.Delay` 10.0)
  (`self.K2_DestroyActor`))

(event `self.Box.OnComponentHit`
  (params (HitComponent :type "PrimitiveComponent Object Reference") (OtherActor :type "Actor Object Reference") (OtherComp :type "PrimitiveComponent Object Reference") (NormalImpulse :type "Vector Structure") (Hit :type "HitResult Structure (by ref)"))
  (bind _ascharacter_enemy (cast `/Game/Blueprints/Characters/Enemies/Character_Enemy` OtherActor))
  (`/Game/Blueprints/Components/CombatComponent.LooseHealth` (`/Game/Blueprints/Characters/Character_Parent.CombatComponent` _ascharacter_enemy) 1)
  (`self.K2_DestroyActor`))

(fn `UserConstructionScript`)