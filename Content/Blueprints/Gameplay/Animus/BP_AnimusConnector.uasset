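; BP_AnimusConnector is an Animus connector actor that visually switches between active and inactive states.
; On BeginPlay it creates a dynamic instance of MI_ConnectorAnim and applies it to the Connector component.
; Activate and Deactivate play the ChangeColorOverTime timeline forward or in reverse, driving the material's Time parameter.
; The timeline's direction sets the Active flag on each update, so the flag flips as the transition starts rather than when it finishes.
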(event `self.ReceiveBeginPlay`
  (bind _returnvalue (`KismetMaterialLibrary.CreateDynamicMaterialInstance` "/Game/Blueprints/Gameplay/Animus/MI_ConnectorAnim.MI_ConnectorAnim"))
  (bind _output_get (set `self.DMI` _returnvalue))
  (`PrimitiveComponent.SetMaterial` (`self.Connector`) 0 _output_get))

(event `Activate`
  (bind (_direction _colorchangevalue) (`Timeline|ChangeColorOverTime` :!via `PlayFromStart` :!label _label)
    (:`Update`
      (`MaterialInstanceDynamic.SetScalarParameterValue` (`self.DMI`) "Time" _colorchangevalue)
      (switch `ETimelineDirection` _direction
        (:`Forward`
          (set `self.Active` true))
        (:`Backward`
          (set `self.Active` false))))))

(event `Deactivate`
  (goto _label :!via `ReverseFromEnd`))

(fn `UserConstructionScript`)