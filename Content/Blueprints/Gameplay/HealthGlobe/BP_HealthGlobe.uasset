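; Health globe pickup that flies to the main character on overlap and restores health.
; Overlapping the sphere destroys the trigger and plays a timeline that lerps the globe toward the player's current position, offset by the mesh height.
; Once within range, a one-shot gate calls the combat component's GetHealth, hides the mesh, activates Niagara and audio effects, and destroys the actor after a short delay.
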(event `self.OverlapSphere.OnComponentBeginOverlap`
  (params (OverlappedComponent :type "PrimitiveComponent Object Reference") (OtherActor :type "Actor Object Reference") (OtherComp :type "PrimitiveComponent Object Reference") (OtherBodyIndex :type Integer) (bFromSweep :type Boolean) (SweepResult :type "HitResult Structure (by ref)"))
  (bind _returnvalue (`self.K2_GetActorLocation`))
  (bind _movetoplayer (`self.MoveToPlayer`))
  (bind (_relativelocation_x _relativelocation_y _relativelocation_z) (`KismetMathLibrary.BreakVector` (`SceneComponent.RelativeLocation` (`self.SphereMesh`))))
  (bind _asmain_character (cast `/Game/Blueprints/Characters/MainCharacter/MainCharacter` OtherActor))
  (`ActorComponent.K2_DestroyComponent` (`self.OverlapSphere`))
  (`Timeline|MoveToPlayer`
    (:`Update`
      (bind _returnvalue_2 (- (`self.K2_GetActorLocation` _asmain_character) (`KismetMathLibrary.MakeVector` 0.0 0.0 _relativelocation_z)))
      (`self.K2_SetActorLocation` (`KismetMathLibrary.VLerp` _returnvalue _returnvalue_2 (`KismetMathLibrary.MapRangeClamped` (`TimelineComponent.GetPlaybackPosition` _movetoplayer) 0.0 (`TimelineComponent.GetTimelineLength` _movetoplayer) 0.0 1.0)))
      (if (== _returnvalue _returnvalue_2 :`ErrorTolerance` 25.0)
        (`/Engine/EditorBlueprintResources/StandardMacros.DoOnce` false
          (:`Completed`
            (`self.GetHealth`)))))))

(event `GetHealth`
  (`/Game/Blueprints/Components/CombatComponent.GetHealth` (`/Game/Blueprints/Characters/Character_Parent.CombatComponent` (stale `self.OverlapSphere.OnComponentBeginOverlap` _asmain_character)) 1)
  (`SceneComponent.SetVisibility` (`self.SphereMesh`) false false)
  (`ActorComponent.Activate` (`self.Niagara`) false)
  (`ActorComponent.Activate` (`self.Audio`) false)
  (`KismetSystemLibrary.Delay` 0.5)
  (`self.K2_DestroyActor`))

(fn `UserConstructionScript`)