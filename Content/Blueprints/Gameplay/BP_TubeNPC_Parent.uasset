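; BP_TubeNPC_Parent is a base Blueprint for interactable tubes that hold an NPC and can be defective.
; Interacting with a valid NPC reference either sets up that NPC's level through the Animus when defective, or releases the NPC.
; Repair clears the defect and saves the tube's class through the TopDownGameMode save object.
; Release also saves, but clears NPCRef before reading its class for the released list.
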(event `self.ReceiveBeginPlay`
  (bind _astop_down_game_mode (cast `/Game/Blueprints/Game/TopDownGameMode` (`GameplayStatics.GetGameMode`)))
  (set `self.Top Down Game Mode` _astop_down_game_mode))

(event `/Game/Blueprints/Interfaces/Interact.Interact`
  (params (PlayerControllerRef :type "/Game/Blueprints/Game/TopDownController Object Reference"))
  (`self.NPC_Ref`
    (:`then`
      (if (`self.Defect`)
        (`self.ActivateAnimus`)
        (else
          (`self.ReleaseNPC`))))
    (:`else`)))

(event `ActivateAnimus`
  (`/Game/Blueprints/Gameplay/Animus/BP_Animus.SetupNPCLevel` (`self.Animus_Ref`) (`self.NPC_Ref`)))

(event `ReleaseNPC`
  (set `self.NPC_Ref` null)
  (`KismetArrayLibrary.Array_AddUnique` (`/Game/Blueprints/Game/SaveGameObject.ReleasedNPCs` (`/Game/Blueprints/Game/TopDownGameMode.SaveGameObject` (`self.Top Down Game Mode`))) (`GameplayStatics.GetObjectClass` (`self.NPC_Ref`)))
  (`/Game/Blueprints/Game/TopDownGameMode.SaveGame` (`self.Top Down Game Mode`)))

(event `RepairTube`
  (set `self.Defect` false)
  (`KismetArrayLibrary.Array_AddUnique` (`/Game/Blueprints/Game/SaveGameObject.RepairedTubes` (`/Game/Blueprints/Game/TopDownGameMode.SaveGameObject` (`self.Top Down Game Mode`))) (`GameplayStatics.GetObjectClass` self))
  (`/Game/Blueprints/Game/TopDownGameMode.SaveGame` (`self.Top Down Game Mode`)))

(fn `UserConstructionScript`)