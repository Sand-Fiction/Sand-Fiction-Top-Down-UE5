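; BP_RelaxBench is an interactable bench that toggles the player between sitting and standing, with a "Sit Down" HUD prompt.
; A FlipFlop on Interact first walks the pawn over, snaps or moves it into alignment, disables movement, plays the sit montage and blends the view to the bench.
; The next interaction restores walking and the player camera, then plays the stand-up montage, using its length as a delay before stopping it.
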(event `/Game/Blueprints/Interfaces/Interact.Interact`
  (params (PlayerControllerRef :type "/Game/Blueprints/Game/MainChar_Controller Object Reference"))
  (bind (_returnvalue_x _returnvalue_y _returnvalue_z) (`KismetMathLibrary.BreakVector` (`self.K2_GetActorLocation`)))
  (bind _characterpawn (`/Game/Blueprints/Game/MainChar_Controller.CharacterPawn` PlayerControllerRef))
  (bind _charactermovement (`Character.CharacterMovement` _characterpawn))
  (`/Engine/EditorBlueprintResources/StandardMacros.FlipFlop`
    (:`A`
      (`AIBlueprintHelperLibrary.SimpleMoveToActor` PlayerControllerRef self)
      (`KismetSystemLibrary.Delay` 1.0)
      (`KismetSystemLibrary.MoveComponentTo` (`Actor.RootComponent` _characterpawn) (`KismetMathLibrary.MakeVector` _returnvalue_x _returnvalue_y (+ _returnvalue_z (`CapsuleComponent.GetScaledCapsuleHalfHeight` (`Character.CapsuleComponent` _characterpawn)))) (`self.K2_GetActorRotation`))
      (`CharacterMovementComponent.SetMovementMode` _charactermovement "MOVE_None" 0)
      (`Character.PlayAnimMontage` (`GameplayStatics.GetPlayerCharacter` 0) "/Game/Assets/Animations/Tobi/FBX/Bench/SitDownBench_Montage.SitDownBench_Montage" 1.0 "None")
      (`PlayerController.SetViewTargetWithBlend` PlayerControllerRef self 3.0 "VTBlend_Linear" 0.0 false))
    (:`B`
      (`/Game/Blueprints/Characters/MFL_Misc.StopCurrentMontage` (`Character.Mesh` _characterpawn))
      (`CharacterMovementComponent.SetMovementMode` _charactermovement "MOVE_Walking" 0)
      (`PlayerController.SetViewTargetWithBlend` PlayerControllerRef (`/Game/Blueprints/Game/MainChar_Controller.CameraRef` PlayerControllerRef) 3.0 "VTBlend_Linear" 0.0 false)
      (bind _returnvalue (`Character.PlayAnimMontage` _characterpawn "/Game/Assets/Animations/Tobi/FBX/Bench/SitUpBench_Montage.SitUpBench_Montage" 1.0 "None"))
      (`KismetSystemLibrary.Delay` _returnvalue)
      (`/Game/Blueprints/Characters/MFL_Misc.StopCurrentMontage` null))))

(event `/Game/Blueprints/Interfaces/Interact.InteractMessage`
  (params (Visible :type Boolean) (`HUD Widget` :type "/Game/Blueprints/UI/WBP_HUD Object Reference"))
  (`/Game/Blueprints/UI/WBP_HUD.DisplayInteractMessage` `HUD Widget` self Visible "Sit Down"))

(fn `UserConstructionScript`)