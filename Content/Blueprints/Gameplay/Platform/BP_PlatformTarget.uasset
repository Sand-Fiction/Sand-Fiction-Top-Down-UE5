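; BP_PlatformTarget is an actor whose mesh disappears and reappears in response to a referenced Platform.
; On BeginPlay it binds its handlers to the Platform's Down and Up events.
; Down hides the static mesh, disables its collision and plays a sound at the actor's location.
; Up restores visibility and query-and-physics collision, with a separate return sound.
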(event `self.ReceiveBeginPlay`
  (bind _platform (`self.Platform`))
  (add `/Game/Blueprints/Gameplay/Platform/BP_Platform.Down` _platform (delegate `DownAction`))
  (add `/Game/Blueprints/Gameplay/Platform/BP_Platform.Up` _platform (delegate `UpAction`)))

(event `DownAction`
  (bind _staticmesh (`self.StaticMesh`))
  (`SceneComponent.SetVisibility` _staticmesh false false)
  (`PrimitiveComponent.SetCollisionEnabled` _staticmesh "NoCollision")
  (`GameplayStatics.PlaySoundAtLocation` "/Game/Sounds/SFX/interior/Cue_platform.Cue_platform" (`self.K2_GetActorLocation`) (struct) 1.0 1.0 0.0 null null null))

(event `UpAction`
  (bind _staticmesh (`self.StaticMesh`))
  (`SceneComponent.SetVisibility` _staticmesh true false)
  (`PrimitiveComponent.SetCollisionEnabled` _staticmesh "QueryAndPhysics")
  (`GameplayStatics.PlaySoundAtLocation` "/Game/Sounds/SFX/interior/cue_platform_back.cue_platform_back" (`self.K2_GetActorLocation`) (struct) 1.0 1.0 0.0 null null null))

(fn `UserConstructionScript`)