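; BP_PuzzlePlatform is a puzzle platform that moves vertically in response to characters entering or leaving its trigger box.
; A Character_Parent overlap plays the PlatformDown timeline, and ending the overlap reverses it.
; Each timeline update sets the platform's relative Z and plays the down or up sound at the actor's location according to direction, so the sound call repeats throughout the movement.
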(event `self.Box.OnComponentBeginOverlap`
  (params (OverlappedComponent :type "PrimitiveComponent Object Reference") (OtherActor :type "Actor Object Reference") (OtherComp :type "PrimitiveComponent Object Reference") (OtherBodyIndex :type Integer) (bFromSweep :type Boolean) (SweepResult :type "HitResult Structure (by ref)"))
  (bind _returnvalue (`self.K2_GetActorLocation`))
  (cast `/Game/Blueprints/Characters/Character_Parent` OtherActor)
  (bind (_direction _zposition) (`Timeline|PlatformDown` :!label _label)
    (:`Update`
      (`SceneComponent.K2_SetRelativeLocation` (`self.Platform`) (`KismetMathLibrary.MakeVector` 0.0 0.0 _zposition) false false)
      (switch `ETimelineDirection` _direction
        (:`Forward`
          (`GameplayStatics.PlaySoundAtLocation` (`self.Sound_PlatformDown`) _returnvalue (struct) 1.0 1.0 0.0 null null null))
        (:`Backward`
          (`GameplayStatics.PlaySoundAtLocation` (`self.Sound_PlatformUp`) _returnvalue (struct) 1.0 1.0 0.0 null null null))))))

(event `self.Box.OnComponentEndOverlap`
  (params (OverlappedComponent :type "PrimitiveComponent Object Reference") (OtherActor :type "Actor Object Reference") (OtherComp :type "PrimitiveComponent Object Reference") (OtherBodyIndex :type Integer))
  (cast `/Game/Blueprints/Characters/Character_Parent` OtherActor)
  (goto _label :!via `Reverse`))

(fn `UserConstructionScript`)