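; BP_Platform is a pressure plate that sinks when a Character_Parent or BP_Pushable enters its box.
; It tracks overlapping actors and drives the platform's height with a timeline, reversing it once the box is empty unless StaysDown is set.
; DoOnce gates play the down and up sounds once per movement.
; CallDown fires when the descent finishes, while CallUp fires as the rise starts.
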(event `self.Box.OnComponentBeginOverlap`
  (params (OverlappedComponent :type "PrimitiveComponent Object Reference") (OtherActor :type "Actor Object Reference") (OtherComp :type "PrimitiveComponent Object Reference") (OtherBodyIndex :type Integer) (bFromSweep :type Boolean) (SweepResult :type "HitResult Structure (by ref)"))
  (bind _returnvalue (`self.K2_GetActorLocation`))
  (if (or (`.bSuccess` (cast `/Game/Blueprints/Characters/Character_Parent` OtherActor :!pure true)) (`.bSuccess` (cast `/Game/Blueprints/Gameplay/BP_Pushable` OtherActor :!pure true)))
    (`KismetArrayLibrary.Array_AddUnique` (`self.Other Actor`) OtherActor)
    (bind (_direction _zposition) (`Timeline|PlatformDown` :!label _label)
      (:`Update`
        (`SceneComponent.K2_SetRelativeLocation` (`self.Platform`) (`KismetMathLibrary.MakeVector` 0.0 0.0 _zposition) false false)
        (switch `ETimelineDirection` _direction
          (:`Forward`
            (`/Engine/EditorBlueprintResources/StandardMacros.DoOnce` false :!label _label_2
              (:`Completed`
                (`GameplayStatics.PlaySoundAtLocation` (`self.Sound_PlatformDown`) _returnvalue (struct) 1.0 1.0 0.0 null null null))))
          (:`Backward`
            (`/Engine/EditorBlueprintResources/StandardMacros.DoOnce` false :!label _label_3
              (:`Completed`
                (`GameplayStatics.PlaySoundAtLocation` (`self.Sound_PlatformUp`) _returnvalue (struct) 1.0 1.0 0.0 null null null)
                (`self.Up`))))))
      (:`Finished`
        (switch `ETimelineDirection` _direction
          (:`Forward`
            (`self.Down`)
            (goto _label_3 :!via `Reset`))
          (:`Backward`
            (goto _label_2 :!via `Reset`)))))))

(event `self.Box.OnComponentEndOverlap`
  (params (OverlappedComponent :type "PrimitiveComponent Object Reference") (OtherActor :type "Actor Object Reference") (OtherComp :type "PrimitiveComponent Object Reference") (OtherBodyIndex :type Integer))
  (bind _other_actor (`self.Other Actor`))
  (`KismetArrayLibrary.Array_RemoveItem` _other_actor OtherActor)
  (if (`KismetArrayLibrary.Array_IsEmpty` _other_actor)
    (if (not (`self.StaysDown`))
      (goto _label :!via `Reverse`))))

(fn `UserConstructionScript`)