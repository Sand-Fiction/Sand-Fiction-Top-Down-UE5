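; A level streaming trigger that swaps sets of levels on overlap and moves the player to a target position.
; On any actor overlap it passes its load and unload lists to SF_GameInstance, then binds to that instance's all-levels-loaded event.
; When that event fires, it teleports player character 0 to the TargetPosition actor's location and rotation, raised by the capsule half height.
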(event `self.ReceiveActorBeginOverlap`
  (params (OtherActor :type "Actor Object Reference"))
  (bind _assf_game_instance (cast `/Game/Blueprints/Game/SF_GameInstance` (`GameplayStatics.GetGameInstance`)))
  (`/Game/Blueprints/Game/SF_GameInstance.LoadLevels` _assf_game_instance (`self.LevelsToLoad`) (`self.LevelsToUnload`))
  (add `/Game/Blueprints/Game/SF_GameInstance.AllLevelsLoaded` _assf_game_instance (delegate `SetCharacterPosition`)))

(event `SetCharacterPosition`
  (bind _returnvalue (`GameplayStatics.GetPlayerCharacter` 0))
  (bind _returnvalue_2 (`self.GetTransform` (`self.TargetPosition`)))
  (`self.K2_SetActorLocationAndRotation` _returnvalue (`KismetMathLibrary.MakeVector` (.x (.location _returnvalue_2)) (.y (.location _returnvalue_2)) (+ (`CapsuleComponent.GetScaledCapsuleHalfHeight` (`Character.CapsuleComponent` _returnvalue)) (.z (.location _returnvalue_2)))) (.rotation _returnvalue_2) false true))

(fn `UserConstructionScript`)