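; Level Sequence director for LS_FadeToBlack that hands off HUD and player input during the sequence.
; One event hides the level HUD and disables input on the first player's pawn, and the other shows the HUD and restores input.
; Both reach the HUD through the first player state's controller and do nothing if the cast to HUD_Level fails.
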(event `SequenceEvent_0`
  (bind _returnvalue (`PlayerState.GetPlayerController` (`GameplayStatics.GetPlayerState` 0)))
  (bind _ashud_level (cast `/Game/Blueprints/Game/HUD_Level` (`PlayerController.GetHUD` _returnvalue)))
  (`/Game/Blueprints/Game/HUD_Level.SetHudVisibility` _ashud_level false)
  (`Actor.DisableInput` (`GameplayStatics.GetPlayerPawn` 0) _returnvalue))

(event `SequenceEvent_1`
  (bind _returnvalue (`PlayerState.GetPlayerController` (`GameplayStatics.GetPlayerState` 0)))
  (bind _ashud_level (cast `/Game/Blueprints/Game/HUD_Level` (`PlayerController.GetHUD` _returnvalue)))
  (`/Game/Blueprints/Game/HUD_Level.SetHudVisibility` _ashud_level true)
  (`Actor.EnableInput` (`GameplayStatics.GetPlayerPawn` 0) _returnvalue))