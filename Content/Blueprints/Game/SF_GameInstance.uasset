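; Game instance that owns the single-slot save object and handles new, save and load game requests.
; Init loads any existing save; NewGame deletes it, creates a fresh object and opens GameplayTest.
; SaveGame writes the held object to disk, while LoadGame only opens Map_HUB without re-reading the slot.
; SavePlayerVariables, which zeroes the saved skill fields, and a slot reload before LoadGame are left unconnected.
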(event `NewGame`
  (`GameplayStatics.DeleteGameInSlot` "Slot01")
  (bind _returnvalue (`GameplayStatics.CreateSaveGameObject` "/Game/Blueprints/Game/SF_SaveGameObject.SF_SaveGameObject_C"))
  (set `self.Save Game Object` _returnvalue)
  (`GameplayStatics.OpenLevelBySoftObjectPtr` "/Game/Maps/Testlevel/GameplayTest.GameplayTest"))

(event `SaveGame`
  (`GameplayStatics.SaveGameToSlot` (`self.Save Game Object`) "Slot01"))

(event `self.ReceiveInit`
  (bind _returnvalue (`GameplayStatics.DoesSaveGameExist` "Slot01"))
  (if _returnvalue
    (bind _returnvalue_2 (`GameplayStatics.LoadGameFromSlot` "Slot01"))
    (bind _assf_save_game_object (cast `/Game/Blueprints/Game/SF_SaveGameObject` _returnvalue_2))
    (set `self.Save Game Object` _assf_save_game_object)))

(event `LoadGame`
  (`GameplayStatics.OpenLevelBySoftObjectPtr` "/Game/Maps/Map_HUB.Map_HUB"))

(fn `SavePlayerVariables`
  (bind _save_game_object (`self.Save Game Object`))
  (cast `/Game/Blueprints/Characters/Character_Parent` (`GameplayStatics.GetPlayerCharacter` 0))
  (set `/Game/Blueprints/Game/SF_SaveGameObject.SkillPoints` 0 _save_game_object)
  (set `/Game/Blueprints/Game/SF_SaveGameObject.SkillsHealth` 0 _save_game_object)
  (set `/Game/Blueprints/Game/SF_SaveGameObject.SkillsMelee` 0 _save_game_object)
  (set `/Game/Blueprints/Game/SF_SaveGameObject.SkillsRanged` 0 _save_game_object))