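; BP_Thunder creates recurring lightning flashes by briefly changing the exposure of a referenced post process volume.
; A self-calling Lightning event, started on BeginPlay, waits a random few seconds before each flash.
; It saves the volume's current exposure compensation, overrides it for a fraction of a second, then restores it and schedules the next flash.
; Despite the name, it plays no thunder sound.
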(event `self.ReceiveBeginPlay`
  (`self.Lightning`))

(event `Lightning`
  (bind _settings (`PostProcessVolume.Settings` (`self.PostProcessingVolume`)))
  (`KismetSystemLibrary.Delay` (`KismetMathLibrary.RandomFloatInRange` 5.0 10.0))
  (bind _output_get (set `self.Default Exposure Compensation` (`.AutoExposureBias` (break `PostProcessSettings` _settings))))
  (bind _structout (setmembers `PostProcessSettings` :`StructRef` _settings :`AutoExposureBias` 7.0))
  (`KismetSystemLibrary.Delay` 0.2)
  (setmembers `PostProcessSettings` :`StructRef` _structout :`AutoExposureBias` _output_get)
  (`self.Lightning`))

(fn `UserConstructionScript`)