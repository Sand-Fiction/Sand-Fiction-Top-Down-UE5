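; Parent actor for lights that flicker by animating the intensity of a point light.
; On BeginPlay it caches the light's starting intensity, sets the Flickering timeline's play rate from a speed variable and plays it from the start.
; The timeline's update multiplies the cached intensity by its IntensityMultiplier track, so the flicker scales with the light's own brightness.
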(event `self.ReceiveBeginPlay`
  (bind _flickering (`self.Flickering`))
  (set `self.Intensity` (`LightComponentBase.Intensity` (`self.PointLight`)))
  (`TimelineComponent.SetPlayRate` _flickering (`self.FlickeringSpeed`))
  (`TimelineComponent.PlayFromStart` _flickering))

(fn `UserConstructionScript`)