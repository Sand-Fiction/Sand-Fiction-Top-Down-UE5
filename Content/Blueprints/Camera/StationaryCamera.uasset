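; StationaryCamera is a placeable camera point with a spring arm and a sphere radius that registers itself with a nearby FollowCamera.
; On BeginPlay it waits a zero-second Delay so the player spawns first, then picks the first FollowCamera found inside the radius.
; Overlap resets that camera to its defaults and sets this actor as its StationaryCamera.
; The construction script applies arm length and sphere radius from variables.
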(event `self.ReceiveBeginPlay`
  (`KismetSystemLibrary.Delay` 0.0) ; Need this to happen after Player Spawn
  (bind _outactors (`GameplayStatics.GetAllActorsOfClass` "/Game/Blueprints/Camera/FollowCamera.FollowCamera_C"))
  (for _array_element _outactors :!label _label
    (if (< (`self.GetDistanceTo` _array_element self) (`self.Sphere Radius`))
      (set `self.Follow Camera` _array_element)
      (`self.Overlap`)
      (`self.BreakLoop`))))

(event `BreakLoop`
  (goto _label :!via `Break`))

(event `Overlap`
  (bind _follow_camera (`self.Follow Camera`))
  (`/Game/Blueprints/Camera/FollowCamera.SetDefaults` _follow_camera)
  (set `/Game/Blueprints/Camera/FollowCamera.Stationary Camera` self _follow_camera))

(fn `UserConstructionScript`
  (set `SpringArmComponent.TargetArmLength` (`self.Arm Length`) (`self.SpringArm`))
  (`SphereComponent.SetSphereRadius` (`self.Sphere`) (`self.Sphere Radius`) true))