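; Player follow camera that becomes the view target at start and uses sphere overlaps to track nearby StationaryCamera actors.
; On entering one, it saves its rotation and arm length.
; A SetCameraLocation update, never triggered in this graph, places it ahead of the player, blending rotation and arm length toward the stationary camera's by player distance over sphere radius, or restoring saved values when none is set.
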(event `self.ReceiveBeginPlay`
  (`PlayerController.SetViewTargetWithBlend` (`GameplayStatics.GetPlayerController` 0) self 0.0 "VTBlend_Linear" 0.0 false)
  (for _array_element (`PrimitiveComponent.GetOverlappingActors` (`self.Sphere`) "/Game/Blueprints/Camera/StationaryCamera.StationaryCamera_C")
    (bind _asstationary_camera (cast `/Game/Blueprints/Camera/StationaryCamera` _array_element))
    (set `self.Stationary Camera` _asstationary_camera)
    (`KismetSystemLibrary.PrintString` "Hello")))

(event `self.Sphere.OnComponentBeginOverlap`
  (params (OverlappedComponent :type "PrimitiveComponent Object Reference") (OtherActor :type "Actor Object Reference") (OtherComp :type "PrimitiveComponent Object Reference") (OtherBodyIndex :type Integer) (bFromSweep :type Boolean) (SweepResult :type "HitResult Structure (by ref)"))
  (bind _asstationary_camera (cast `/Game/Blueprints/Camera/StationaryCamera` OtherActor))
  (set `self.Stationary Camera` _asstationary_camera)
  (set `self.Rotation Before Entering` (`self.K2_GetActorRotation`))
  (set `self.Arm Length Before Entering` (`SpringArmComponent.TargetArmLength` (`self.SpringArm`))))

(event `self.Sphere.OnComponentEndOverlap`
  (params (OverlappedComponent :type "PrimitiveComponent Object Reference") (OtherActor :type "Actor Object Reference") (OtherComp :type "PrimitiveComponent Object Reference") (OtherBodyIndex :type Integer))
  (cast `/Game/Blueprints/Camera/StationaryCamera` OtherActor)
  (set `self.Stationary Camera` null))

(fn `GetPlayerCameraPosition`
  (returns (ReturnValue :type "Vector Structure"))
  (bind _returnvalue (`GameplayStatics.GetPlayerPawn` 0))
  (return (+ (`self.K2_GetActorLocation` _returnvalue) (* (`self.GetActorForwardVector` _returnvalue) (`self.CameraDistanceInFrontOfPlayer`)))))

(fn `UserConstructionScript`
  (bind _output_get (set `self.Default Arm Length` (`SpringArmComponent.TargetArmLength` (`self.SpringArm`))))
  (set `self.Arm Length Before Entering` _output_get))