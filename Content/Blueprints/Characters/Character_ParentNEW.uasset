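; Parent character Blueprint that provides shared health, death and walk/run speed logic.
; Healing, damage and max-health increases update the health values and fire the UpdateHealth dispatcher, with current health clamped on healing and damage.
; Zero health triggers Death through a DoOnce, which the base Death event immediately resets via ResetDeath.
; Attack, ResetAttack, GetHit and SnapRotation are empty events, apparently hooks for child classes.
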(event `self.ReceiveBeginPlay`
  ;[1 1 1] Initialize
)

(event `Walk`
  ;[1 1 1] Movement Speed
  (set `CharacterMovementComponent.MaxWalkSpeed` (`self.WalkSpeed`) (`self.CharacterMovement`)))

(event `GetHealth`
  (params (Health :type Integer))
  ;[1 1 1] Health / Death
  (set `self.HealthCurrent` (`KismetMathLibrary.Clamp` (+ (`self.HealthCurrent`) Health) 0 (`self.HealthMax`)))
  (`self.UpdateHealth`))

(event `Run`
  ;[1 1 1] Movement Speed
  (set `CharacterMovementComponent.MaxWalkSpeed` (`self.RunSpeed`) (`self.CharacterMovement`)))

(event `LooseHealth`
  (params (Damage :type Integer))
  ;[1 1 1] Health / Death
  (bind _output_get (set `self.HealthCurrent` (`KismetMathLibrary.Clamp` (- (`self.HealthCurrent`) Damage) 0 (`self.HealthMax`))))
  (`self.UpdateHealth`)
  (if (== _output_get 0)
    (`/Engine/EditorBlueprintResources/StandardMacros.DoOnce` false :!label _label
      (:`Completed`
        (`self.Death`)))))

(event `Attack`
  ;[1 1 1] Combat
)

(event `ResetDeath`
  ;[1 1 1] Health / Death
  (goto _label :!via `Reset`))

(event `Reset Attack`
  ;[1 1 1] Combat
)

(event `Death`
  ;[1 1 1] Health / Death
  (`self.ResetDeath`))

(event `GetHit`
  ;[1 1 1] Combat
)

(event `IncreaseMaximumHealth`
  (params (HealthIncrease :type Integer))
  ;[1 1 1] Health / Death
  (set `self.HealthMax` (+ HealthIncrease (`self.HealthMax`)))
  (`self.UpdateHealth`))

(event `SnapRotation`
  ;[1 1 1] Rotation
)

(fn `UserConstructionScript`)