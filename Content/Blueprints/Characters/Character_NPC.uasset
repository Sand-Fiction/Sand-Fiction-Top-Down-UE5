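; Character Blueprint for an NPC that the player can interact with to start a dialogue.
; Interact calls TalkToPlayer, which, if CanTalkTo is set, opens the dialogue window on the level HUD widget and passes itself as the speaker.
; It then plays the RotateToPlayer timeline, whose update smoothly turns the NPC toward the player character.
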(event `/Game/Blueprints/Interfaces/Interact.Interact`
  (params (PlayerControllerRef :type "/Game/Blueprints/Game/MainChar_Controller Object Reference"))
  (`self.TalkToPlayer`))

(event `TalkToPlayer`
  (if (`self.CanTalkTo`)
    (bind _ashud_level (cast `/Game/Blueprints/Game/HUD_Level` (`PlayerController.GetHUD` (`GameplayStatics.GetPlayerController` 0))))
    (`/Game/Blueprints/UI/WBP_HUD.TriggerDialogueWindow` (`/Game/Blueprints/Game/HUD_Level.HUD Widget` _ashud_level) true self)
    (`TimelineComponent.PlayFromStart` (`self.RotateToPlayer`))))

(fn `UserConstructionScript`
  (`parent.UserConstructionScript`))