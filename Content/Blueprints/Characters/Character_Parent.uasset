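; Base character for the main character, NPCs and enemies, handling health, armor, melee combat, dialogue interaction and death.
; Attacks sphere-trace for hostile characters, then apply blocking or random damage with crits, feeding armor-first health loss, damage numbers, knockback and time-dilation hit stop.
; A CharacterType enum branches health bar setup, armor blinking, interaction and death: the main character respawns at PlayerStart, while others are destroyed.
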(event `ActivateArmor`
  (bind _armorparticles (`self.ArmorParticles`))
  ;[1 1 1] ArmorParticles
  (`/Engine/EditorBlueprintResources/StandardMacros.DoOnce` false :!label _label
    (:`Completed`
      (`ActorComponent.Deactivate` _armorparticles)
      (`KismetSystemLibrary.Delay` 0.1)
      (`ActorComponent.Activate` _armorparticles false)
      (`KismetSystemLibrary.Delay` 1.0)
      (`self.ResetArmorActivation`))))

(event `ResetArmorActivation`
  ;[1 1 1] ArmorParticles
  (goto _label :!via `Reset`))

(event `self.ReceiveBeginPlay`
  ;[1 1 1] Initialize
  (`self.Initialize Healthbar`)
  (`NiagaraComponent.SetVariableFloat` (`self.ArmorParticles`) "ArmorUptime" (`self.ArmorUptime`)))

(event `GetHealth`
  (params (Health :type Integer))
  ;[1 1 1] Health
  (set `self.HealthCurrent` (`KismetMathLibrary.Clamp` (+ Health (`self.HealthCurrent`)) 0 (`self.HealthMax`)))
  (`self.UpdateHealth`))

(event `/Game/Blueprints/Interfaces/Interact.Interact`
  (params (PlayerControllerRef :type "/Game/Blueprints/Game/MainChar_Controller Object Reference"))
  ;[1 1 1] Dialogue
  (if (`self.CanInteract`)
    (switch `/Game/Blueprints/Characters/E_CharacterType` (`self.CharacterType`)
      (:`NewEnumerator1`
        (bind _ashud_level (cast `/Game/Blueprints/Game/HUD_Level` (`PlayerController.GetHUD` (`GameplayStatics.GetPlayerController` 0))))
        (`/Game/Blueprints/UI/WBP_HUD.TriggerDialogueWindow` (`/Game/Blueprints/Game/HUD_Level.HUD Widget` _ashud_level) true self)
        (`TimelineComponent.PlayFromStart` (`self.Rotate to Player`))))))

(event `GetArmor`
  (params (Armor :type Integer))
  ;[1 1 1] Health
  (set `self.Armor` (`KismetMathLibrary.Clamp` (+ Armor (`self.Armor`)) 0 (`self.HealthCurrent`)))
  (`self.UpdateHealth`)
  (`KismetSystemLibrary.RetriggerableDelay` (- (`self.ArmorUptime`) 3.0))
  (`self.LooseArmorAfterTime`))

(event `LooseArmorAfterTime`
  ;[1 1 1] Health
  (switch `/Game/Blueprints/Characters/E_CharacterType` (`self.CharacterType`)
    (:`NewEnumerator0`
      (bind _asmain_char_controller (cast `/Game/Blueprints/Game/MainChar_Controller` (`self.GetController`)))
      (`/Game/Blueprints/UI/WBP_HealthBar.BlinkArmor` (`/Game/Blueprints/UI/WBP_HUD.WBP_PlayerHealth` (`/Game/Blueprints/Game/MainChar_Controller.HUDWidget` _asmain_char_controller))))
    (:`NewEnumerator1`
      (bind _aswbp_health_bar (cast `/Game/Blueprints/UI/WBP_HealthBar` (`WidgetComponent.GetWidget` (`self.Widget`)) :!label _label_2))
      (`/Game/Blueprints/UI/WBP_HealthBar.BlinkArmor` _aswbp_health_bar))
    (:`NewEnumerator2`
      (goto _label_2)))
  (`KismetSystemLibrary.Delay` 2.0)
  (`GameplayStatics.PlaySoundAtLocation` "/Game/Sounds/SFX/interior/Cue_stone_armor_end.Cue_stone_armor_end" (`self.K2_GetActorLocation`) (struct) 1.0 1.0 0.0 null null null null)
  (`KismetSystemLibrary.Delay` 1.0)
  (set `self.Armor` 0)
  (`self.UpdateHealth`))

(event `/Game/Blueprints/Interfaces/Interact.InteractMessage`
  (params (Visible :type Boolean) (`HUD Widget` :type "/Game/Blueprints/UI/WBP_HUD Object Reference"))
  ;[1 1 1] Dialogue
  (if (`self.CanInteract`)
    (switch `/Game/Blueprints/Characters/E_CharacterType` (`self.CharacterType`)
      (:`NewEnumerator1`
        (`/Game/Blueprints/UI/WBP_HUD.DisplayInteractMessage` `HUD Widget` self Visible (`|FormatText` "Talk to {Name}" (`self.Name`)))))))

(event `Walk`
  ;[1 1 1] Movement Speed
  (set `CharacterMovementComponent.MaxWalkSpeed` (`self.WalkSpeed`) (`self.CharacterMovement`)))

(event `LooseHealth`
  (params (Damage :type Integer))
  (bind _returnvalue (- (`self.Armor`) Damage))
  ;[1 1 1] Health
  (if (> (`self.Armor`) 0)
    (if (< _returnvalue 0)
      (set `self.HealthCurrent` (`KismetMathLibrary.Clamp` (- (`self.HealthCurrent`) (`KismetMathLibrary.Abs_Int` _returnvalue)) 0 (`self.HealthMax`)))
      (set `self.Armor` 0)
      (`ActorComponent.Deactivate` (`self.ArmorParticles`))
      (else
        (set `self.Armor` (`KismetMathLibrary.Clamp` _returnvalue 0 (`self.HealthCurrent`)))))
    (`self.UpdateHealth`)
    (else
      (bind _output_get (set `self.HealthCurrent` (`KismetMathLibrary.Clamp` (- (`self.HealthCurrent`) Damage) 0 (`self.HealthMax`))))
      (`self.UpdateHealth`)
      (if (== _output_get 0)
        (`/Engine/EditorBlueprintResources/StandardMacros.DoOnce` false :!label _label_3
          (:`Completed`
            (`self.Death`)))))))

(event `CannotTalkInFight`
  ;[1 1 1] Dialogue
  (set `self.CanInteract` false)
  (`KismetSystemLibrary.RetriggerableDelay` 3.0)
  (set `self.CanInteract` true))

(event `Run`
  ;[1 1 1] Movement Speed
  (set `CharacterMovementComponent.MaxWalkSpeed` (`self.RunSpeed`) (`self.CharacterMovement`)))

(event `ResetDeath`
  ;[1 1 1] Health
  (goto _label_3 :!via `Reset`))

(event `SnapRotation`
  ;[1 1 1] Rotation
)

(event `IncreaseMaximumHealth`
  (params (HealthIncrease :type Integer))
  ;[1 1 1] Health
  (set `self.HealthMax` (+ HealthIncrease (`self.HealthMax`)))
  (`self.UpdateHealth`))

(event `Respawn`
  (bind _returnvalue (`GameplayStatics.GetPlayerController` 0))
  ;[1 1 1] Respawn
  (`MovementComponent.StopMovementImmediately` (`self.CharacterMovement`))
  (`|ExecutionSequence`
    (:`then_0`
      (bind _assf_game_instance (cast `/Game/Blueprints/Game/SF_GameInstance` (`GameplayStatics.GetGameInstance`)))
      (bind _save_game_object (`/Game/Blueprints/Game/SF_GameInstance.Save Game Object` _assf_game_instance)
        (:`then`
          (`/Game/Blueprints/Game/SF_SaveGameObject.Checkpoint` _save_game_object
            (:`then`
              _)
            (:`else`
              _)))
        (:`else`
          _))
      (bind _returnvalue_2 (`GameplayStatics.GetActorOfClass` "/Script/Engine.PlayerStart"))
      (`self.K2_SetActorLocation` (`self.K2_GetActorLocation` _returnvalue_2)))
    (:`then_1`
      (`self.GetHealth` (`self.HealthMax`))
      (`PrimitiveComponent.SetCollisionEnabled` (`self.CapsuleComponent`) "QueryAndPhysics")
      (`|PlayMontage` (`self.Mesh`) "/Game/Template/Mixamo/SwordAndShield_Retargeted/sword_and_shield_power_up_Montage.sword_and_shield_power_up_Montage" 1.25
        (:`then`
          (`WidgetBlueprintLibrary.SetInputMode_UIOnlyEx` _returnvalue null)
          (`self.SetActorTickEnabled` _returnvalue false))
        (:`OnCompleted`
          (`WidgetBlueprintLibrary.SetInputMode_GameAndUIEx` _returnvalue null "DoNotLock" false :!label _label_4)
          (`self.SetActorTickEnabled` _returnvalue true))
        (:`OnInterrupted`
          (goto _label_4))))))

(event `Death`
  ;[1 1 1] Death
  (`self.CharacterDeath`)
  (`PrimitiveComponent.SetCollisionEnabled` (`self.CapsuleComponent`) "NoCollision")
  (`self.ResetDeath`)
  (`SceneComponent.SetVisibility` (`self.Widget`) false false)
  (`/Game/Blueprints/Characters/MFL_Misc.StopCurrentMontage` (`self.Mesh`))
  (`CharacterMovementComponent.DisableMovement` (`self.CharacterMovement`))
  (`KismetSystemLibrary.Delay` 0.05)
  (`|PlayMontage` (`self.Mesh`) (`self.Death_Montage`)
    (:`OnCompleted`
      (switch `/Game/Blueprints/Characters/E_CharacterType` (`self.CharacterType`)
        (:`NewEnumerator0`
          (`self.Respawn`))
        (:`NewEnumerator1`
          (`self.K2_DestroyActor` :!label _label_5))
        (:`NewEnumerator2`
          (goto _label_5))))))

(event `AttackCheck`
  ;[1 1 1] Combat
  (`self.CannotTalkInFight`)
  (bind _charactershit (`self.TraceForEnemies` 50.0))
  (for _array_element _charactershit
    (`/Engine/EditorBlueprintResources/StandardMacros.IsValid` _array_element
      (:`Is Valid`
        (if (and (`/Game/Blueprints/Characters/Character_Parent.isBlocking` _array_element) (not (`/Game/Blueprints/Characters/MFL_Misc.CheckDotProductActors` _array_element self)))
          (`self.BlockHit` _array_element)
          (`self.BlockHit`)
          (else
            (`self.GetHit` _array_element self)))))))

(event `/Game/Blueprints/Interfaces/Shootable.GetShot`
  (params (Arrow :type "/Game/Blueprints/Combat/BP_RangedProjectile Object Reference"))
  ;[1 1 1] Combat
  (bind _characterparent (`/Game/Blueprints/Combat/BP_RangedProjectile.CharacterParent` Arrow)
    (:`then`
      (`self.GetHit` _characterparent))
    (:`else`)))

(event `GetHit`
  (params (Character :type "/Game/Blueprints/Characters/Character_Parent Object Reference"))
  ;[1 1 1] Combat
  (`self.CannotTalkInFight`)
  (if (and (!= (`self.HealthCurrent`) 0) (not (`self.isDodging`)))
    (bind (_damage _crit) (`self.CalculateDamage` Character))
    (`self.Receive Damage` _damage _crit)
    (`AISense_Damage.ReportDamageEvent` self Character (`KismetMathLibrary.Conv_IntToDouble` _damage) (`self.K2_GetActorLocation` Character))
    (if (not (`NavMovementComponent.IsFalling` (`self.CharacterMovement`)))
      (`TimelineComponent.PlayFromStart` (`self.Knockback`))
      (`self.HitStop` Character _damage)
      (`CharacterMovementComponent.DisableMovement` (`self.CharacterMovement`))
      (`|PlayMontage` (`self.Mesh`) (`self.GetHit_Montage`) 1.5
        (:`OnCompleted`
          _)
        (:`OnInterrupted`
          _))
      (`CharacterMovementComponent.SetMovementMode` (`self.CharacterMovement`) "MOVE_Walking" 0))))

(event `Receive Damage`
  (params (Damage :type Integer) (Crit :type Boolean))
  (bind (_returnvalue_x _returnvalue_y _returnvalue_z) (`KismetMathLibrary.BreakVector` (`self.K2_GetActorLocation`)))
  ;[1 1 1] Combat
  (`self.LooseHealth` Damage)
  (`|SpawnActorFromClass` "/Game/Blueprints/Combat/BP_DamageNumber.BP_DamageNumber_C" (`KismetMathLibrary.MakeTransform` (`KismetMathLibrary.MakeVector` (+ _returnvalue_x (`KismetMathLibrary.RandomFloatInRange` -25.0 25.0)) (+ _returnvalue_y (`KismetMathLibrary.RandomFloatInRange` -25.0 25.0)) (+ _returnvalue_z 200.0))) "Undefined" "OverrideRootScale" null Damage Crit null)
  (`NiagaraFunctionLibrary.SpawnSystemAtLocation` "/Game/VFX/NE_HitEffect_System.NE_HitEffect_System" (`self.K2_GetActorLocation`)))

(event `GroundSlam`
  ;[1 1 1] Combat
  (`self.CannotTalkInFight`)
  (bind _charactershit (`self.TraceForEnemies` 250.0 true))
  (for _array_element _charactershit
    (`/Engine/EditorBlueprintResources/StandardMacros.IsValid` _array_element
      (:`Is Valid`
        (`self.GetHit` _array_element self)))))

(event `BlockHit`
  (bind _charactermovement (`self.CharacterMovement`))
  ;[1 1 1] Combat
  (`CharacterMovementComponent.DisableMovement` _charactermovement)
  (`|PlayMontage` (`self.Mesh`) (`self.BlockHit_Montage`) 1.5
    (:`OnCompleted`
      _)
    (:`OnInterrupted`
      _))
  (`CharacterMovementComponent.SetMovementMode` _charactermovement "MOVE_Walking" 0))

(event `HitStop`
  (params (OtherCharacter :type "/Game/Blueprints/Characters/Character_Parent Object Reference") (Damage :type Integer))
  ;[1 1 1] Combat
  (set `Actor.CustomTimeDilation` 0.1 OtherCharacter)
  (set `self.CustomTimeDilation` 0.1)
  (`KismetSystemLibrary.Delay` (* Damage (`self.HitStopModifier`) 0.1))
  (set `Actor.CustomTimeDilation` 1.0 OtherCharacter)
  (set `self.CustomTimeDilation` 1.0))

(fn `CalculateDamage`
  (params (Enemy :type "/Game/Blueprints/Characters/Character_Parent Object Reference"))
  (returns (Damage :type Integer) (Crit :type Boolean))
  (locals (Critical :type Boolean) (ActualDamage :type Integer))
  (bind _output_get (set `local.ActualDamage` (`KismetMathLibrary.RandomIntegerInRange` (`/Game/Blueprints/Characters/Character_Parent.DamageMin` Enemy) (`/Game/Blueprints/Characters/Character_Parent.DamageMax` Enemy))))
  (bind _output_get_2 (set `local.Critical` (>= (`self.CriticalStrikeChance`) (`KismetMathLibrary.RandomIntegerInRange` 1 100))))
  (return (`KismetMathLibrary.SelectInt` (* _output_get 2) _output_get _output_get_2) _output_get_2))

(fn `HideHealthBarBasedOnDistance`
  (`SceneComponent.SetHiddenInGame` (`self.Widget`) (> (`self.GetDistanceTo` (`GameplayStatics.GetPlayerCharacter` 0) self) 1000.0) false))

(fn `Initialize Healthbar`
  (switch `/Game/Blueprints/Characters/E_CharacterType` (`self.CharacterType`)
    (:`NewEnumerator1`
      (bind _aswbp_health_bar (cast `/Game/Blueprints/UI/WBP_HealthBar` (`WidgetComponent.GetUserWidgetObject` (`self.Widget`)) :!label _label))
      (`/Game/Blueprints/UI/WBP_HealthBar.Bind Healthbar` _aswbp_health_bar self))
    (:`NewEnumerator2`
      (`|ExecutionSequence`
        (:`then_0`
          (goto _label))
        (:`then_1`
          (`KismetSystemLibrary.K2_SetTimer` null "HideHealthBarBasedOnDistance" 0.5 true))))))

(fn `TraceForEnemies`
  (params (Radius :type "Float (single-precision)") (Sphere :type Boolean))
  (returns (CharactersHit :type "Array of /Game/Blueprints/Characters/Character_Parent Object Reference"))
  (locals (HitArray :type "Array of /Game/Blueprints/Characters/Character_Parent Object Reference"))
  (bind _returnvalue (`self.K2_GetActorLocation`))
  (bind (_outhits _returnvalue_2) (`KismetSystemLibrary.SphereTraceMultiForObjects` _returnvalue (`KismetMathLibrary.SelectVector` _returnvalue (+ _returnvalue (* (`self.GetActorForwardVector`) (`self.AttackRange`))) Sphere) Radius (`|MakeArray` "ObjectTypeQuery3" :!type "EObjectTypeQuery Enum")))
  (if _returnvalue_2
    (for _array_element _outhits
      (bind _ascharacter_parent (cast `/Game/Blueprints/Characters/Character_Parent` (`.HitActor` (`GameplayStatics.BreakHitResult` _array_element))))
      (bind _hostile (`/Game/Blueprints/Characters/MFL_Misc.Check Character Hostility` self _ascharacter_parent))
      (if _hostile
        (`KismetArrayLibrary.Array_AddUnique` (`local.HitArray`) _ascharacter_parent))))
  (return (`local.HitArray`)))

(fn `UserConstructionScript`
  (switch `/Game/Blueprints/Characters/E_CharacterType` (`self.CharacterType`)
    (:`NewEnumerator0`
      (set `self.AIControllerClass` "/Game/Blueprints/Game/MainChar_Controller.MainChar_Controller_C"))
    (:`NewEnumerator1`
      (set `self.AIControllerClass` "/Game/Blueprints/Characters/Enemies/AI_Controller.AI_Controller_C" :!label _label))
    (:`NewEnumerator2`
      (goto _label))))