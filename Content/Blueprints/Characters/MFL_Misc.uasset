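; A miscellaneous Blueprint library of small helpers for actors and characters.
; RotateActorToPlayer smoothly turns an actor's yaw toward player 0 with RInterpTo and a look-at rotation, keeping its pitch and roll.
; CheckDotProductActors compares two actors' forward vectors, returning the dot product and whether it is non-negative.
; StopCurrentMontage stops a skeletal mesh's active montage using a given blend-out time.
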(fn `CheckDotProductActors`
  (params (Actor01 :type "Actor Object Reference") (Actor02 :type "Actor Object Reference"))
  (returns (Positive :type Boolean) (DotProduct :type "Float (double-precision)"))
  (bind _returnvalue (`KismetMathLibrary.Dot_VectorVector` (`Actor.GetActorForwardVector` Actor01) (`Actor.GetActorForwardVector` Actor02)))
  (return (>= _returnvalue 0.0) _returnvalue))

(fn `RotateActorToPlayer`
  (params (Actor :type "Actor Object Reference") (InterpSpeed :type "Float (double-precision)"))
  (bind _returnvalue (`Actor.K2_GetActorRotation` Actor))
  (bind ___worldcontext (`local.__WorldContext`))
  (`Actor.K2_SetActorRotation` Actor (`KismetMathLibrary.MakeRotator` (.roll _returnvalue) (.pitch _returnvalue) (.yaw (`KismetMathLibrary.RInterpTo` _returnvalue (`KismetMathLibrary.FindLookAtRotation` (`Actor.K2_GetActorLocation` Actor) (`Actor.K2_GetActorLocation` (`GameplayStatics.GetPlayerCharacter` ___worldcontext))) (`GameplayStatics.GetWorldDeltaSeconds` ___worldcontext) InterpSpeed))) false))

(fn `StopCurrentMontage`
  (params (`Skeletal Mesh` :type "SkeletalMeshComponent Object Reference") (InBlendOutTime :type "Float (double-precision)"))
  (bind _returnvalue (`SkeletalMeshComponent.GetAnimInstance` `Skeletal Mesh`))
  (`AnimInstance.Montage_Stop` _returnvalue InBlendOutTime (`AnimInstance.GetCurrentActiveMontage` _returnvalue))
  (return))