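; Parent Blueprint for human characters, handling melee and ranged weapon draw, sheath and switching, plus snapping rotation to the mouse through MainChar_Controller.
; On BeginPlay it caches the melee, shield and ranged child actors as BP_WeaponParent references.
; Draw and sheath call Appear or Dissolve by WeaponMode, using paired DoOnce gates that reset each other, with sheath starting closed.
; Switching sheathes the current set, toggles the mode, then draws the other.
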(event `self.ReceiveBeginPlay`
  ;[1 1 1] Important
  (`parent.ReceiveBeginPlay`)
  (`self.SaveWeaponActorRefs`))

(event `self.SnapRotation`
  (bind _asmain_char_controller (cast `/Game/Blueprints/Game/MainChar_Controller` (`self.GetController` self)))
  (`/Game/Blueprints/Game/MainChar_Controller.RotateToMouse` _asmain_char_controller))

(event `DrawWeapons`
  ;[1 1 1] Weapon Draw/Sheath/Switch
  (`/Engine/EditorBlueprintResources/StandardMacros.DoOnce` false :!label _label
    (:`Completed`
      (switch `/Game/Blueprints/Combat/WeaponMode` (`self.WeaponMode`)
        (:`NewEnumerator0`
          (`/Game/Blueprints/Combat/Weapons/BP_WeaponParent.Appear` (`self.MeleeWeaponActor`))
          (`/Game/Blueprints/Combat/Weapons/BP_WeaponParent.Appear` (`self.ShieldWeaponActor`)))
        (:`NewEnumerator1`
          (`/Game/Blueprints/Combat/Weapons/BP_WeaponParent.Appear` (`self.RangedWeaponActor`))))
      (`self.ResetSheathWeapons`))))

(event `ResetDrawWeapons`
  ;[1 1 1] Weapon Draw/Sheath/Switch
  (goto _label :!via `Reset`))

(event `SheathWeapons`
  ;[1 1 1] Weapon Draw/Sheath/Switch
  (`/Engine/EditorBlueprintResources/StandardMacros.DoOnce` true :!label _label_2
    (:`Completed`
      (switch `/Game/Blueprints/Combat/WeaponMode` (`self.WeaponMode`)
        (:`NewEnumerator0`
          (`/Game/Blueprints/Combat/Weapons/BP_WeaponParent.Dissolve` (`self.MeleeWeaponActor`))
          (`/Game/Blueprints/Combat/Weapons/BP_WeaponParent.Dissolve` (`self.ShieldWeaponActor`)))
        (:`NewEnumerator1`
          (`/Game/Blueprints/Combat/Weapons/BP_WeaponParent.Dissolve` (`self.RangedWeaponActor`))))
      (`self.ResetDrawWeapons`))))

(event `ResetSheathWeapons`
  ;[1 1 1] Weapon Draw/Sheath/Switch
  (goto _label_2 :!via `Reset`))

(event `SwitchWeapons`
  ;[1 1 1] Weapon Draw/Sheath/Switch
  (`self.SheathWeapons`)
  (switch `/Game/Blueprints/Combat/WeaponMode` (`self.WeaponMode`)
    (:`NewEnumerator0`
      (set `self.WeaponMode` "NewEnumerator1"))
    (:`NewEnumerator1`
      (set `self.WeaponMode` "NewEnumerator0")))
  (`self.DrawWeapons`))

(fn `SaveWeaponActorRefs`
  (bind _asbp_weapon_parent (cast `/Game/Blueprints/Combat/Weapons/BP_WeaponParent` (`ChildActorComponent.ChildActor` (`self.MeleeWeapon`))))
  (set `self.MeleeWeaponActor` _asbp_weapon_parent)
  (bind _asbp_weapon_parent_2 (cast `/Game/Blueprints/Combat/Weapons/BP_WeaponParent` (`ChildActorComponent.ChildActor` (`self.Shield`))))
  (set `self.ShieldWeaponActor` _asbp_weapon_parent_2)
  (bind _asbp_weapon_parent_3 (cast `/Game/Blueprints/Combat/Weapons/BP_WeaponParent` (`ChildActorComponent.ChildActor` (`self.RangedWeapon`))))
  (set `self.RangedWeaponActor` _asbp_weapon_parent_3))

(fn `UserConstructionScript`
  (`parent.UserConstructionScript`))