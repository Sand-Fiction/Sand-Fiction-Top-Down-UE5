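; Combat component that tracks an owner's health in the game.
; LooseHealth subtracts damage from CurrentHealth and GetHealth adds health to it.
; Both events clamp the result between zero and MaxHealth, and nothing in the graph reacts when health reaches zero.
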(event `LooseHealth`
  (params (Damage :type Integer))
  (set `self.CurrentHealth` (`KismetMathLibrary.Clamp` (- (`self.CurrentHealth`) Damage) 0 (`self.MaxHealth`))))

(event `GetHealth`
  (params (Health :type Integer))
  (set `self.CurrentHealth` (`KismetMathLibrary.Clamp` (+ (`self.CurrentHealth`) Health) 0 (`self.MaxHealth`))))